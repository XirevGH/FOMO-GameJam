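; BP_GameMode is a game mode that sets up two local players when play begins.
; It spawns a BP_PlayerCharacter at each of the first two PlayerStarts found in the level.
; The existing first controller possesses one; a newly created local player possesses the other, which spawns with ControllerIndex set.
; A single WBP_Minimap is added to the viewport during the second player's setup.
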(event `self.ReceiveBeginPlay`
  (bind _outactors (`GameplayStatics.GetAllActorsOfClass` "/Script/Engine.PlayerStart"))
  (for _index (range 2)
    (if (> _index 0)
      (bind _returnvalue (`GameplayStatics.CreatePlayer` -1))
      (bind _returnvalue_2 (`self.GetTransform` (`|GetArrayItem` _outactors _index)))
      (bind _returnvalue_3 (`|SpawnActorFromClass` "/Game/Blueprints/BP_PlayerCharacter.BP_PlayerCharacter_C" _returnvalue_2 "Undefined" "MultiplyWithRoot" null 1 null))
      (`Controller.Possess` _returnvalue _returnvalue_3)
      (bind _returnvalue_4 (`|CreateWidget` "/Game/UI/WBP_Minimap.WBP_Minimap_C"))
      (`UserWidget.AddToViewport` _returnvalue_4 0)
      (else
        (bind _returnvalue_5 (`|SpawnActorFromClass` "/Game/Blueprints/BP_PlayerCharacter.BP_PlayerCharacter_C" _returnvalue_2 "Undefined" "MultiplyWithRoot" null 0 null))
        (`Controller.Possess` (`GameplayStatics.GetPlayerController` 0) _returnvalue_5)))))

(fn `UserConstructionScript`)