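; BP_SpeedPickUp is a pickup actor, named for a speed boost, that only animates itself: it spins and bobs.
; Each Tick adds a fixed yaw step, so spin rate depends on frame rate, then applies the location computed by AnimateHeight.
; AnimateHeight accumulates delta time into a sine wave that drives Z while keeping X and Y.
; BeginPlay and overlap events are disabled, so no boost or collection logic exists here.
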(event `self.ReceiveTick`
  (params (DeltaSeconds :type "Float (single-precision)"))
  (bind (_returnvalue_roll _returnvalue_pitch _returnvalue_yaw) (`KismetMathLibrary.BreakRotator` (`self.K2_GetActorRotation` self)))
  (`self.K2_SetActorRotation` self (`KismetMathLibrary.MakeRotator` 0.0 0.0 (+ 3.0 _returnvalue_yaw)) false)
  (bind (_self2 _returnvalue_x _returnvalue_y _returnvalue) (`self.AnimateHeight`))
  (`self.K2_SetActorLocation` _self2 (`KismetMathLibrary.MakeVector` _returnvalue_x _returnvalue_y _returnvalue) false false))

(fn `AnimateHeight`
  (returns (self2 :type "Self Object Reference") (ReturnValue_X :type "Float (double-precision)") (ReturnValue_Y :type "Float (double-precision)") (ReturnValue :type "Float (double-precision)"))
  (bind (_returnvalue_x _returnvalue_y) (`KismetMathLibrary.BreakVector` (`self.K2_GetActorLocation` self)))
  (bind _output_get (set `self.TimeAccumulator` (+ (`GameplayStatics.GetWorldDeltaSeconds`) (`self.TimeAccumulator`))))
  (return self _returnvalue_x _returnvalue_y (+ (+ (* (`KismetMathLibrary.DegSin` (* _output_get 300.0)) 30.0) (`self.New Location Y`)) 115.0)))

(fn `UserConstructionScript`
  (`parent.UserConstructionScript`))