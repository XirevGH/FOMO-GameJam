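; Player character for a multi-player setup that registers itself with a shared controller when it is the second player.
; On possession it adds the default Enhanced Input mapping context, then, if the controller index is 1, stores itself as Player2 on the first BP_SharedController found.
; Every tick it resets its text render to a fixed world rotation, so the text does not turn with the character.
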(event `self.ReceivePossessed`
  (params (NewController :type "Controller Object Reference"))
  (bind _asplayer_controller (cast `PlayerController` (`self.GetController`)))
  (bind _returnvalue (pcsubsystem `EnhancedInputLocalPlayerSubsystem` _asplayer_controller))
  (`/Engine/EditorBlueprintResources/StandardMacros.IsValid` _returnvalue
    (:`Is Valid`
      (`EnhancedInputSubsystemInterface.AddMappingContext` _returnvalue "/Game/Inputs/IMC_Default.IMC_Default" 0 (struct))
      (if (== 1 (`self.ControllerIndex`))
        (bind _outactors (`GameplayStatics.GetAllActorsOfClass` "/Game/Blueprints/BP_SharedController.BP_SharedController_C"))
        (set `/Game/Blueprints/BP_SharedController.Player2` self (`|GetArrayItem` _outactors))))))

(event `self.ReceiveTick`
  (params (DeltaSeconds :type "Float (single-precision)"))
  (`SceneComponent.K2_SetWorldRotation` (`self.TextRender`) (struct :`Pitch` 90.0 :`Yaw` 270.0 :`Roll` 90.0) false false))

(fn `UserConstructionScript`)