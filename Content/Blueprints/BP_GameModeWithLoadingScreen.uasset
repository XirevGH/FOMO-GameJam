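; Game mode that shows a loading screen at BeginPlay while it spawns two local player characters at PlayerStart locations.
; A two-pass loop spawns and possesses each BP_PlayerCharacter, creating a second local player for the second one.
; The first player's input is disabled for a fixed delay, independent of actual load progress.
; After the delay, that input returns and the minimap widget replaces the loading screen.
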(event `self.ReceiveBeginPlay`
  (bind _returnvalue (`|CreateWidget` "/Game/Blueprints/WB_LoadingScreenWidget.WB_LoadingScreenWidget_C"))
  (`UserWidget.AddToViewport` _returnvalue 0)
  (bind _outactors (`GameplayStatics.GetAllActorsOfClass` "/Script/Engine.PlayerStart"))
  (for _index (range 2)
    (if (> _index 0)
      (bind _returnvalue_2 (`GameplayStatics.CreatePlayer` -1))
      (bind _returnvalue_3 (`self.GetTransform` (`|GetArrayItem` _outactors _index)))
      (bind _returnvalue_4 (`|SpawnActorFromClass` "/Game/Blueprints/BP_PlayerCharacter.BP_PlayerCharacter_C" _returnvalue_3 "Undefined" "MultiplyWithRoot" null 1 null))
      (`Controller.Possess` _returnvalue_2 _returnvalue_4)
      (else
        (bind _returnvalue_5 (`|SpawnActorFromClass` "/Game/Blueprints/BP_PlayerCharacter.BP_PlayerCharacter_C" _returnvalue_3 "Undefined" "MultiplyWithRoot" null 0 null))
        (`Controller.Possess` (`GameplayStatics.GetPlayerController` 0) _returnvalue_5)
        (`self.DisableInput` (`GameplayStatics.GetPlayerCharacter` 0) (`GameplayStatics.GetPlayerController` 0))
        (`KismetSystemLibrary.Delay` 20.0)
        (`self.EnableInput` (`GameplayStatics.GetPlayerCharacter` 0) (`GameplayStatics.GetPlayerController` 0))
        (`Widget.RemoveFromParent` _returnvalue)
        (bind _returnvalue_6 (`|CreateWidget` "/Game/UI/WBP_Minimap.WBP_Minimap_C"))
        (`UserWidget.AddToViewport` _returnvalue_6 0)))))

(fn `UserConstructionScript`)